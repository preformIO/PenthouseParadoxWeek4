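; BP_LVL_Changer is a level transition actor that moves the player to the level chosen by its LevelName enum.
; When BP_MysteryChar overlaps the LevelUpward_Trigger, it shows a W_LevelTrans widget, plays its screen transition, then opens the level after a short delay.
; The enum's string doubles as the level name to open and as the NextLevel text set in the construction script.
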(event OnComponentBeginOverlap(LevelUpward_Trigger)
  (params (OverlappedComponent :type Primitive%20Component%20Object%20Reference) (OtherActor :type Actor%20Object%20Reference) (OtherComp :type Primitive%20Component%20Object%20Reference) (OtherBodyIndex :type Integer) (bFromSweep :type Boolean) (SweepResult :type Hit%20Result%20Structure%20%28by%20ref%29))
  (bind _level_name (Variables|Default|GetLevel%20Name))
  (bind _returnvalue (Utilities|String|EnumtoString _level_name))
  (Utilities|Casting|CastToBP_MysteryChar OtherActor)
  (Development|PrintString (Utilities|String|Append "Loading level: " _returnvalue))
  (bind _returnvalue_2 (UserInterface|CreateWidget "/Game/Widgets/W_LevelTrans.W_LevelTrans_C"))
  (UserInterface|Viewport|AddtoViewport _returnvalue_2 0)
  (Default|ScreenLvlTransition _returnvalue_2)
  (Utilities|FlowControl|Delay 1.0)
  (Game|OpenLevel(byName) (Utilities|String|StringToName _returnvalue)))

(event EventBeginPlay)

(event Collision|EventActorBeginOverlap
  (params (OtherActor :type Actor%20Object%20Reference)))

(event EventTick
  (params (DeltaSeconds :type Float%20%28single-precision%29)))

(fn ConstructionScript
  (Rendering|Components|TextRender|SetText (Variables|Default|GetNextLevel) (Utilities|Text|ToText(String) (Utilities|String|EnumtoString (Variables|Default|GetLevel%20Name)))))