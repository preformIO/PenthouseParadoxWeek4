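; BP_SplineMesh_Instance is a construction-script tool that repeats a chosen static mesh along a spline as instances.
; Spacing is the mesh's X bounds plus DistanceOffset, and the spline length divided by that spacing sets how many instances are placed.
; Each instance can optionally face the next point along the spline, and the InstancedStaticMesh component gets query and physics collision.
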(event EventBeginPlay)

(event Collision|EventActorBeginOverlap
  (params (OtherActor :type Actor%20Object%20Reference)))

(event EventTick
  (params (DeltaSeconds :type Float%20%28single-precision%29)))

(fn ConstructionScript
  (bind _mesh (Variables|Default|GetMesh))
  (bind _instancedstaticmesh (Variables|Default|GetInstancedStaticMesh))
  (bind _returnvalue (StaticMesh|GetBoundingBox _mesh))
  (bind (_min _max) (Utilities|Struct|BreakBox _returnvalue))
  (Components|StaticMesh|SetStaticMesh (Variables|Default|GetInstancedStaticMesh) (Variables|Default|GetMesh))
  (bind _output_get (Variables|Default|SetSpace (+ (.X (Class|KismetMathLibrary|BreakVector3f (- _max _min))) (Variables|Default|GetDistanceOffset))))
  ;[1 1 1] How many?
  (bind _output_get_2 (LocalVariables|SetInstancesNumber (Math|Float|Floor (/ (Spline|GetSplineLength (Variables|Default|GetSpline)) _output_get))))
  (for _index (range 0 _output_get_2)
    (Components|InstancedStaticMesh|AddInstance _instancedstaticmesh (Math|Transform|MakeTransform (CallFunction|GetLocationatIndex _index) (select (Variables|Default|GetUseRotation?) (Math|Conversions|RotationFromXVector (- (CallFunction|GetLocationatIndex (+ _index 1)) (CallFunction|GetLocationatIndex _index))) "0, 0, 0")) false)
    (Collision|SetCollisionEnabled _instancedstaticmesh "QueryAndPhysics")))

(fn GetLocationatIndex
  (params (Index :type Integer))
  (return (Spline|GetLocationatDistanceAlongSpline (Variables|Default|GetSpline) (* Index (Variables|Default|GetSpace)) "Local")))