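; Health component that stores a current health value and changes it within minimum and maximum bounds.
; AddHealth and RemoveHealth add or subtract an amount, clamp the result and return it.
; UpdateHealth routes positive changes to AddHealth and others to RemoveHealth unnegated, so negative changes also raise health, then prints the value on screen for debugging.
; BeginPlay and Tick are unused.
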(event EventBeginPlay)

(event EventTick
  (params (DeltaSeconds :type Float%20%28single-precision%29)))

(fn RemoveHealth
  (params (Amount :type Float%20%28double-precision%29))
  (bind _output_get (Variables|Default|SetCurrentHealth (Math|Float|Clamp(Float) (- (Variables|Default|GetCurrentHealth) Amount) (Variables|Default|GetMinHealth) (Variables|Default|GetMaxHealth))))
  ;[1 1 1] check this
  (return _output_get))

(fn AddHealth
  (params (Amount :type Float%20%28double-precision%29))
  (bind _output_get (Variables|Default|SetCurrentHealth (Math|Float|Clamp(Float) (+ (Variables|Default|GetCurrentHealth) Amount) (Variables|Default|GetMinHealth) (Variables|Default|GetMaxHealth))))
  (return _output_get))

(fn UpdateHealth
  (params (HealthAmountChange :type Float%20%28double-precision%29))
  (if (> HealthAmountChange 0.0)
    (bind _health (CallFunction|AddHealth HealthAmountChange))
    (Variables|Default|SetCurrentHealth _health)
    (else
      (bind _health_2 (CallFunction|RemoveHealth HealthAmountChange))
      (bind _output_get (Variables|Default|SetCurrentHealth _health_2))))
  (Development|PrintString (Utilities|String|ToString(Float) (Variables|Default|GetCurrentHealth)) true true "(R=0.000000,G=0.660000,B=1.000000,A=1.000000)" 5.0)
  (return _output_get))