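; BP_HiddenDoor is a switch-driven barrier that opens a hidden room once the required number of switches is active.
; BarrierActivated and BarrierDeactivated maintain the active count; an exact match plays Barrier_TL, while other counts and any deactivation reverse it.
; The timeline's Alpha directly sets the barrier's relative roll.
; Unconnected leftover logic includes a duplicate count check and a delayed vertical slide.
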(event Custom|BarrierActivated
  (Math|Integer|IncrementInt (Variables|Default|GetNumSwitchActive)
    (:%20%20
      (if (== (Variables|Default|GetNumSwitchActive) (Variables|Default|GetNumSwitchNeeded))
        (bind _alpha (Timeline|Barrier_TL Play)
          (:Update
            (Transformation|SetRelativeRotation (Variables|Default|GetHiddenRoomBarrier) (Math|Rotator|MakeRotator _alpha 0.0 0.0) false false)))
        (else
          (Timeline|Barrier_TL Reverse))))))

(event Custom|BarrierDeactivated
  (Math|Integer|DecrementInt (Variables|Default|GetNumSwitchActive)
    (:%20%20
      (bind _alpha (Timeline|Barrier_TL Reverse)
        (:Update
          (Transformation|SetRelativeRotation (Variables|Default|GetHiddenRoomBarrier) (Math|Rotator|MakeRotator _alpha 0.0 0.0) false false))))))

(event EventBeginPlay
  ;[1 1 1] debugging
)

(event EventTick
  (params (DeltaSeconds :type Float%20%28single-precision%29))
  ;[1 1 1] debugging
)

(fn ConstructionScript)